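; BP_Item is a pickup actor that carries an Item value for the inventory.
; PickUpItem prints a debug message, triggers the DestroyItem event and returns Item to the caller.
; DestroyItem removes the actor after a short delay.
; When IsKey is set, Tick spins the actor by a fixed local rotation each frame, independent of delta time.
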(event Custom|Destroy%20Item
  (Utilities|FlowControl|Delay 0.1)
  (Actor|DestroyActor))

(event EventBeginPlay)

(event Collision|EventActorBeginOverlap
  (params (OtherActor :type Actor%20Object%20Reference)))

(event EventTick
  (params (DeltaSeconds :type Float%20%28single-precision%29))
  (if (Variables|Default|GetIsKey)
    (Transformation|AddActorLocalRotation "0.000000,5.000000,0.000000" false false)))

(fn ConstructionScript)

(fn PickUpItem
  (Development|PrintString "Item picked!")
  (CallFunction|DestroyItem)
  (return (Variables|Default|Getitem)))