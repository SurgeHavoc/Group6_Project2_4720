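; Inventory component that stores collected items and keeps the inventory UI in sync.
; Adding or removing an item updates the Inventory collection, then casts the owner to BP_CameraManager to update the list in its InventoryWidget.
; A lookup function reports whether a given item is held.
; Additions are also printed to screen for debugging.
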(fn AddItemtoInventory
  (params (NewItem :type String%20%28by%20ref%29))
  (Utilities|Array|Add (Variables|Default|GetInventory) NewItem)
  (Development|PrintString NewItem)
  (bind _asbp_camera_manager (Utilities|Casting|CastToBP_CameraManager (Components|GetOwner)))
  (Default|AddItemtoListUI (Variables|/Game/Blueprints/BP_CameraManager.BP_CameraManager_C|GetInventoryWidget _asbp_camera_manager) NewItem))

(fn CheckInventoryforItem
  (params (ItemToCheck :type String))
  (return (Utilities|Array|ContainsItem (Variables|Default|GetInventory) ItemToCheck)))

(fn RemoveItemfromInventory
  (params (ItemToRemove :type String))
  (Utilities|Array|RemoveItem (Variables|Default|GetInventory) ItemToRemove)
  (bind _asbp_camera_manager (Utilities|Casting|CastToBP_CameraManager (Components|GetOwner)))
  (Default|RemoveItemfromListUI (Variables|/Game/Blueprints/BP_CameraManager.BP_CameraManager_C|GetInventoryWidget _asbp_camera_manager) ItemToRemove))