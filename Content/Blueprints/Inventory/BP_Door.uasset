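; BP_Door is a key-locked door that moves the player to the next level.
; On BeginPlay it picks the destination from the current level name, cycling Tutorial, Study_Map, Lab_Map and back to Tutorial.
; CheckForKey looks up the given item in the inventory component on BP_CameraManager.
; If found, OpenDoor loads that level by object reference; otherwise a printed message says a key is needed.
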(event Custom|OpenDoor
  (Game|OpenLevel(byObjectReference) (Variables|Default|GetLevel)))

(event EventBeginPlay
  (bind _returnvalue (Game|GetCurrentLevelName true))
  (if (Utilities|Enum|Equal(Enum) _returnvalue "Tutorial")
    (Variables|Default|SetLevel "/Game/Maps/Study_Map.Study_Map")
    (elif (Utilities|Enum|Equal(Enum) _returnvalue "Study_Map")
      (Variables|Default|SetLevel "/Game/Maps/Lab_Map.Lab_Map")
      (elif (Utilities|Enum|Equal(Enum) _returnvalue "Lab_Map")
        (Variables|Default|SetLevel "/Game/Maps/Tutorial.Tutorial")))))

(event Collision|EventActorBeginOverlap
  (params (OtherActor :type Actor%20Object%20Reference)))

(event EventTick
  (params (DeltaSeconds :type Float%20%28single-precision%29)))

(fn ConstructionScript)

(fn CheckforKey
  (params (ItemToCheck :type String))
  (bind _returnvalue (Actor|GetActorOfClass "/Game/Blueprints/BP_CameraManager.BP_CameraManager_C"))
  (bind _hasitem (Default|CheckInventoryforItem (Variables|/Game/Blueprints/BP_CameraManager.BP_CameraManager_C|GetBPC_Inventory _returnvalue) ItemToCheck))
  (if _hasitem
    (CallFunction|OpenDoor)
    (return ItemToCheck)
    (else
      (Development|PrintString "You need a key to open this door!"))))