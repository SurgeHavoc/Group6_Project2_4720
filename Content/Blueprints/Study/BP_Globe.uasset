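; BP_Globe is a clickable puzzle globe that reveals a hidden key when rotated in the correct left/right order.
; Clicking the left or right detector turns the sphere 45 degrees, records the direction and triggers CheckSequence, while hovering sets flags on BP_CameraManager.
; Once the recorded length matches the answer set at BeginPlay, a match tilts the referenced bust head and enables the key; any attempt then clears.
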(event OnClicked(RightDetect)
  (params (TouchedComponent :type Primitive%20Component%20Object%20Reference) (ButtonPressed :type Key%20Structure :default "None"))
  (CallFunction|RotateRight))

(event OnBeginCursorOver(LeftDetect)
  (params (TouchedComponent :type Primitive%20Component%20Object%20Reference))
  (bind _returnvalue (Actor|GetActorOfClass "/Game/Blueprints/BP_CameraManager.BP_CameraManager_C"))
  (Variables|/Game/Blueprints/BP_CameraManager.BP_CameraManager_C|SetIsHoveringLeftGlobe? _returnvalue true))

(event OnClicked(LeftDetect)
  (params (TouchedComponent :type Primitive%20Component%20Object%20Reference) (ButtonPressed :type Key%20Structure :default "None"))
  (CallFunction|RotateLeft))

(event OnEndCursorOver(LeftDetect)
  (params (TouchedComponent :type Primitive%20Component%20Object%20Reference))
  (bind _returnvalue (Actor|GetActorOfClass "/Game/Blueprints/BP_CameraManager.BP_CameraManager_C"))
  (Variables|/Game/Blueprints/BP_CameraManager.BP_CameraManager_C|SetIsHoveringLeftGlobe? _returnvalue false))

(event OnBeginCursorOver(RightDetect)
  (params (TouchedComponent :type Primitive%20Component%20Object%20Reference))
  (bind _returnvalue (Actor|GetActorOfClass "/Game/Blueprints/BP_CameraManager.BP_CameraManager_C"))
  (Variables|/Game/Blueprints/BP_CameraManager.BP_CameraManager_C|SetIsHoveringRightGlobe? _returnvalue true))

(event OnEndCursorOver(RightDetect)
  (params (TouchedComponent :type Primitive%20Component%20Object%20Reference))
  (bind _returnvalue (Actor|GetActorOfClass "/Game/Blueprints/BP_CameraManager.BP_CameraManager_C"))
  (Variables|/Game/Blueprints/BP_CameraManager.BP_CameraManager_C|SetIsHoveringRightGlobe? _returnvalue false))

(event Custom|RotateRight
  (Transformation|AddRelativeRotation (Variables|Default|GetGlobeSphere) "0.000000,45.000000,0.000000" false false)
  (Development|PrintString "Rotate Right!")
  (Utilities|Array|Add (Variables|Default|GetRotationSequence) 1)
  (for _array_element (Variables|Default|GetRotationSequence)
    (Development|PrintString (Utilities|String|ToString(Integer) _array_element))
    (CallFunction|CheckSequence)))

(event Custom|RotateLeft
  (Transformation|AddRelativeRotation (Variables|Default|GetGlobeSphere) "0.000000,-45.000000,0.000000" false false)
  (Development|PrintString "Rotate Left!")
  (Utilities|Array|Add (Variables|Default|GetRotationSequence) 0)
  (for _array_element (Variables|Default|GetRotationSequence)
    (Development|PrintString (Utilities|String|ToString(Integer) _array_element))
    (CallFunction|CheckSequence)))

(event EventBeginPlay
  (bind _keyreference (Variables|Default|GetKeyReference))
  (bind _output_get (Variables|Default|SetRotationSequence (Variables|Default|GetRotationSequence)))
  (Utilities|Array|Clear _output_get)
  (bind _output_get_2 (Variables|Default|SetCorrectSequence (Utilities|Array|MakeArray (Variables|Default|GetNum) 0 1 1 0 1)))
  (for _array_element _output_get_2
    (Development|PrintString (Utilities|String|ToString(Integer) _array_element))
    (Rendering|SetActorHiddenInGame _keyreference true)
    (Collision|SetActorEnableCollision _keyreference false)))

(event Collision|EventActorBeginOverlap
  (params (OtherActor :type Actor%20Object%20Reference)))

(event EventTick
  (params (DeltaSeconds :type Float%20%28single-precision%29)))

(fn ConstructionScript)

(fn CheckSequence
  (bind _keyreference (Variables|Default|GetKeyReference))
  ;[1 1 1] Check if the length of the arrays match.
  (if (== (Utilities|Array|Length (Variables|Default|GetRotationSequence)) (Utilities|Array|Length (Variables|Default|GetCorrectSequence)))
    (Variables|Default|SetIsSequenceCorrect? true)
    ;[1 1 1] Loop through sequence to check for any rogue elements.
    (for (_array_element _array_index) (Variables|Default|GetRotationSequence)
      (if (not (== (Utilities|Array|Get(acopy) (Variables|Default|GetCorrectSequence) _array_index) _array_element))
        (Utilities|Array|Clear (Variables|Default|GetRotationSequence))
        (Variables|Default|SetIsSequenceCorrect? false)))
    ;[1 1 1] Check if sequence is correct.
    (if (Variables|Default|GetIsSequenceCorrect?)
      (Utilities|Array|Clear (Variables|Default|GetRotationSequence))
      (Development|PrintString "Correct!")
      (Transformation|AddRelativeRotation (Variables|/Script/Engine.Actor|GetRootComponent (Variables|Default|GetBust%20Head%20Reference)) "0.000000,0.000000,45.000000" false false)
      (Rendering|SetActorHiddenInGame _keyreference false)
      (Collision|SetActorEnableCollision _keyreference true)
      (else
        (Utilities|Array|Clear (Variables|Default|GetRotationSequence))
        (Development|PrintString "Try again!")))))