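; BP_Note is a note Blueprint that shows and dismisses a note text widget on screen.
; OpenNote plays a paper sound, then either creates WBP_NoteText and adds it to the viewport or makes the stored widget visible, depending on CreatedWidget.
; CreatedWidget is never set in these graphs.
; CloseNote delegates to the stored widget's own CloseNote, and neither event is triggered within this Blueprint.
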(event Custom|OpenNote
  (if (Variables|Default|GetCreatedWidget?)
    (Audio|PlaySound2D "/Game/Audio/paper-collect-1-186598.paper-collect-1-186598" 1.0 1.0 0.0 0 0)
    (Widget|SetVisibility (Variables|Default|GetNoteReference) "Visible")
    (else
      (Audio|PlaySound2D "/Game/Audio/paper-collect-1-186598.paper-collect-1-186598" 1.0 1.0 0.0 0 0)
      (bind _returnvalue (UserInterface|CreateWidget "/Game/Blueprints/Study/WBP_NoteText.WBP_NoteText_C"))
      (bind _output_get (Variables|Default|SetNoteReference _returnvalue))
      (UserInterface|Viewport|AddtoViewport _output_get 0))))

(event Custom|CloseNote
  (Default|CloseNote (Variables|Default|GetNoteReference)))

(event EventBeginPlay)

(event Collision|EventActorBeginOverlap
  (params (OtherActor :type Actor%20Object%20Reference)))

(event EventTick
  (params (DeltaSeconds :type Float%20%28single-precision%29)))

(fn ConstructionScript)