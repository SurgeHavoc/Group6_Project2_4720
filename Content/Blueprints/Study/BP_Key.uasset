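; BP_Key is a key pickup actor that spins briefly when play begins and can be picked up.
; Tick rotates the mesh each frame until a Delay clears the Spin flag about 1.5 seconds in.
; PickUpItem prints a message, triggers DestroyItem to remove the actor after a short delay, and returns its Item to the caller.
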(event Custom|Destroy%20Item
  (Utilities|FlowControl|Delay 0.1)
  (Actor|DestroyActor))

(event EventBeginPlay
  (Variables|Default|SetSpin? true))

(event Collision|EventActorBeginOverlap
  (params (OtherActor :type Actor%20Object%20Reference)))

(event EventTick
  (params (DeltaSeconds :type Float%20%28single-precision%29))
  (if (Variables|Default|GetSpin?)
    (Transformation|AddLocalRotation (Variables|Default|GetStaticMesh) "0.000000,10.000000,0.000000" false false)
    (Utilities|FlowControl|Delay 1.5)
    (Variables|Default|SetSpin? false)))

(fn ConstructionScript)

(fn PickUpItem
  (Development|PrintString "Item picked!")
  (CallFunction|DestroyItem)
  (return (Variables|Default|Getitem)))