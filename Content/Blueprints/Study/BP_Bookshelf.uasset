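; BP_Bookshelf is an interactive study bookshelf that drops a hidden record after being shaken three times.
; The ShakeShakeShake event rocks the Bookshelf component side to side with timed local rotations, using CanClick to block input until the wobble finishes.
; A click counter caps the shakes; on the third it sets Launch and spawns BP_Record at the Scene component's location.
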(event Custom|ShakeShakeShake
  (if (Variables|Default|GetCanClick?)
    (if (not (>= (Variables|Default|GetClickCount) 3))
      (Variables|Default|SetCanClick? false)
      (Math|Integer|IncrementInt (Variables|Default|GetClickCount)
        (:%20%20
          (Transformation|AddLocalRotation (Variables|Default|GetBookshelf) "10.000000,0.000000,0.000000" false false)
          (Utilities|FlowControl|Delay 0.2)
          (Transformation|AddLocalRotation (Variables|Default|GetBookshelf) "-10.000000,0.000000,0.000000" false false)
          (Utilities|FlowControl|Delay 0.2)
          (Transformation|AddLocalRotation (Variables|Default|GetBookshelf) "-10.000000,0.000000,0.000000" false false)
          (Utilities|FlowControl|Delay 0.2)
          (Transformation|AddLocalRotation (Variables|Default|GetBookshelf) "10.000000,0.000000,0.000000" false false)
          (Variables|Default|SetCanClick? true)
          (if (>= (Variables|Default|GetClickCount) 3)
            (Variables|Default|SetLaunch? true)
            (Game|SpawnActorfromClass "/Game/Blueprints/Study/BP_Record.BP_Record_C" (Math|Transform|MakeTransform (Transformation|GetWorldLocation (Variables|Default|GetScene))) "Undefined" "MultiplyWithRoot" 0 0)))))))

(event EventBeginPlay)

(event Collision|EventActorBeginOverlap
  (params (OtherActor :type Actor%20Object%20Reference)))

(event EventTick
  (params (DeltaSeconds :type Float%20%28single-precision%29)))

(fn ConstructionScript)