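; BP_Gramophone is an interactable gramophone that gives the player a key when they have the required record.
; CheckForItem queries the inventory component on BP_CameraManager, then either triggers InteractWithGramophone and returns the item, or prints that a record is needed.
; InteractWithGramophone spawns a BP_Key at the gramophone's location only once, stores it as the drawer key reference, and launches it upward with a mesh impulse.
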(event Custom|InteractWithGramophone
  (if (not (Variables|Default|GetBHasSpawned))
    (bind _returnvalue (Game|SpawnActorfromClass "/Game/Blueprints/Study/BP_Key.BP_Key_C" (Math|Transform|MakeTransform (Transformation|GetActorLocation)) "Undefined" "MultiplyWithRoot" 0 0))
    (bind _output_get (Variables|Default|SetDrawerKeyReference _returnvalue))
    (Variables|Default|SetBHasSpawned true)
    (Physics|AddImpulse (Variables|/Game/Blueprints/Study/BP_Key.BP_Key_C|GetStaticMesh _output_get) "0.000000,0.000000,3000.000000" "None" false)))

(event EventBeginPlay)

(event Collision|EventActorBeginOverlap
  (params (OtherActor :type Actor%20Object%20Reference)))

(event EventTick
  (params (DeltaSeconds :type Float%20%28single-precision%29)))

(fn ConstructionScript)

(fn CheckforItem
  (params (ItemToCheck :type String))
  (bind _returnvalue (Actor|GetActorOfClass "/Game/Blueprints/BP_CameraManager.BP_CameraManager_C"))
  (bind _hasitem (Default|CheckInventoryforItem (Variables|/Game/Blueprints/BP_CameraManager.BP_CameraManager_C|GetBPC_Inventory _returnvalue) ItemToCheck))
  (if _hasitem
    (CallFunction|InteractwithGramophone)
    (return ItemToCheck)
    (else
      (Development|PrintString "A record is needed!"))))