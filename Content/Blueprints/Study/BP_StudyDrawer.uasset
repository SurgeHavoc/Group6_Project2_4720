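; Lockable study drawer that opens when the required item is in the player's inventory and reveals a note.
; CheckForItem queries the inventory on BP_CameraManager while locked, otherwise toggles the drawer open or closed by offsetting its cube.
; Unlocking calls InteractWithDrawer, which slides it out, then after a short delay spawns BP_Note once at the Scene component with a small upward impulse.
; Hovering the cursor prints a description.
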(event OnBeginCursorOver(Cube)
  (params (TouchedComponent :type Primitive%20Component%20Object%20Reference))
  (Development|PrintString "A drawer."))

(event Custom|InteractWithDrawer
  (Variables|Default|SetIsLocked? false)
  (Transformation|AddRelativeLocation (Variables|Default|GetCube) "0.000000,50.000000,0.000000" false false)
  (Variables|Default|SetBIsMoved? true)
  (Utilities|FlowControl|Delay 0.2)
  (if (not (Variables|Default|GetBHasSpawned))
    (bind _returnvalue (Game|SpawnActorfromClass "/Game/Blueprints/Study/BP_Note.BP_Note_C" (Math|Transform|MakeTransform (Transformation|GetWorldLocation (Variables|Default|GetScene))) "Undefined" "MultiplyWithRoot" 0 0))
    (bind _output_get (Variables|Default|SetStudyNoteReference _returnvalue))
    (Variables|Default|SetBHasSpawned true)
    (Physics|AddImpulse (Variables|/Game/Blueprints/Study/BP_Note.BP_Note_C|GetNote _output_get) "0.000000,0.000000,2.000000" "None" false)))

(event EventBeginPlay)

(event Collision|EventActorBeginOverlap
  (params (OtherActor :type Actor%20Object%20Reference)))

(event EventTick
  (params (DeltaSeconds :type Float%20%28single-precision%29)))

(fn ConstructionScript)

(fn CheckforItem
  (params (ItemToCheck :type String))
  (if (Variables|Default|GetIsLocked?)
    (bind _returnvalue (Actor|GetActorOfClass "/Game/Blueprints/BP_CameraManager.BP_CameraManager_C"))
    (bind _hasitem (Default|CheckInventoryforItem (Variables|/Game/Blueprints/BP_CameraManager.BP_CameraManager_C|GetBPC_Inventory _returnvalue) ItemToCheck))
    (if _hasitem
      (CallFunction|InteractwithDrawer)
      (return ItemToCheck)
      (else
        (Development|PrintString "A key is needed!")))
    (elif (Variables|Default|GetBIsMoved?)
      (Transformation|AddRelativeLocation (Variables|Default|GetCube) "0.000000,-50.000000,0.000000" false false)
      (Variables|Default|SetBIsMoved? false)
      (else
        (Transformation|AddRelativeLocation (Variables|Default|GetCube) "0.000000,50.000000,0.000000" false false)
        (Variables|Default|SetBIsMoved? true)))))