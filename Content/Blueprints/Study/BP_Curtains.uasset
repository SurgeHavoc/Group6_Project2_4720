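; BP_Curtains is an interactive pair of study curtains that slide apart and can be tied open to reveal a hidden text actor.
; CheckForFlowers queries the BP_CameraManager inventory for the given item, locking and tying the curtains if found, otherwise printing a hint and toggling their position.
; Tying swaps meshes and materials and shows the ties.
; A separate event slides unlocked curtains back when the camera manager's Camera 1 is inactive.
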(event Custom|InteractWithCurtains
  (if (Variables|Default|GetIsMoved?)
    _
    (else
      (CallFunction|MoveCurtains)))
  (Rendering|SetActorHiddenInGame (Variables|Default|GetHiddenTextReference) false)
  (Components|StaticMesh|SetStaticMesh (Variables|Default|GetCurtain) "/Game/Meshes/Study/curtainTiedL.curtainTiedL")
  (Rendering|Material|SetMaterial (Variables|Default|GetCurtain) 0 "/Game/Materials/Study/curtainsTied-Study.curtainsTied-Study")
  (Components|StaticMesh|SetStaticMesh (Variables|Default|GetOtherCurtain) "/Game/Meshes/Study/curtainTiedR.curtainTiedR")
  (Rendering|Material|SetMaterial (Variables|Default|GetOtherCurtain) 0 "/Game/Materials/Study/curtainsTied-Study.curtainsTied-Study")
  (Rendering|SetVisibility (Variables|Default|GetcurtainTie) true false)
  (Rendering|SetVisibility (Variables|Default|GetOthercurtainTie) true false))

(event Custom|IsPlayerAway?
  (if (Variables|Default|GetIsMoved?)
    (bind _returnvalue (Actor|GetActorOfClass "/Game/Blueprints/BP_CameraManager.BP_CameraManager_C"))
    (if (not (Variables|/Game/Blueprints/BP_CameraManager.BP_CameraManager_C|GetIsCamera1Active? _returnvalue))
      (if (not (Variables|Default|GetIsLocked?))
        (CallFunction|MoveBackCurtains)))))

(event Custom|MoveBackCurtains
  (Transformation|SetRelativeLocation (Variables|Default|GetCurtain) "0.000000,0.000000,50.000000" false false)
  (Transformation|SetRelativeLocation (Variables|Default|GetOtherCurtain) "0.000000,0.000000,50.000000" false false)
  (Variables|Default|SetIsMoved? false))

(event Custom|MoveCurtains
  (Transformation|AddRelativeLocation (Variables|Default|GetCurtain) "-30.000000,0.000000,0.000000" false false)
  (Transformation|AddRelativeLocation (Variables|Default|GetOtherCurtain) "30.000000,0.000000,0.000000" false false)
  (Variables|Default|SetIsMoved? true))

(event EventBeginPlay)

(event Collision|EventActorBeginOverlap
  (params (OtherActor :type Actor%20Object%20Reference)))

(event EventTick
  (params (DeltaSeconds :type Float%20%28single-precision%29)))

(fn ConstructionScript)

(fn CheckforFlowers
  (params (ItemToCheck :type String))
  (bind _returnvalue (Actor|GetActorOfClass "/Game/Blueprints/BP_CameraManager.BP_CameraManager_C"))
  (bind _hasitem (Default|CheckInventoryforItem (Variables|/Game/Blueprints/BP_CameraManager.BP_CameraManager_C|GetBPC_Inventory _returnvalue) ItemToCheck))
  (if _hasitem
    (Variables|Default|SetIsLocked? true)
    (CallFunction|InteractwithCurtains)
    (return ItemToCheck)
    (else
      (Development|PrintString "Hmm... what could help with these curtains?")
      (if (not (Variables|Default|GetIsLocked?))
        (if (Variables|Default|GetIsMoved?)
          (CallFunction|MoveBackCurtains)
          (else
            (CallFunction|MoveCurtains)))))))