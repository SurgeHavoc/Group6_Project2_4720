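; BP_CrackedBottle is a lab prop that breaks open when the inventory holds the required item, meant to be a hammer.
; CheckForHammer queries the inventory component on BP_CameraManager for the passed item, then either triggers the break and returns that item or prints a hint that a hammer is needed.
; Breaking plays a shatter sound at the bottle's location and destroys the actor after a short delay.
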(event Custom|BreakOpenGlassJug
  (Audio|PlaySoundatLocation "/Game/Audio/Bottle_Break.Bottle_Break" (Transformation|GetActorLocation) "0, 0, 0" 1.0 1.0 0.0 0 0 0 0)
  (Utilities|FlowControl|Delay 0.1)
  (Actor|DestroyActor))

(event EventBeginPlay)

(event Collision|EventActorBeginOverlap
  (params (OtherActor :type Actor%20Object%20Reference)))

(event EventTick
  (params (DeltaSeconds :type Float%20%28single-precision%29)))

(fn ConstructionScript)

(fn CheckforHammer
  (params (ItemToCheck :type String))
  (bind _returnvalue (Actor|GetActorOfClass "/Game/Blueprints/BP_CameraManager.BP_CameraManager_C"))
  (bind _hasitem (Default|CheckInventoryforItem (Variables|/Game/Blueprints/BP_CameraManager.BP_CameraManager_C|GetBPC_Inventory _returnvalue) ItemToCheck))
  (if _hasitem
    (CallFunction|BreakOpenGlassJug)
    (return ItemToCheck)
    (else
      (Development|PrintString "You need a hammer to crack open this cracked bottle!"))))