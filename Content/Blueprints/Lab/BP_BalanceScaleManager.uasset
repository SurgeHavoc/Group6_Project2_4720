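; Manager actor for a lab balance scale puzzle that reacts when the player holds a specific creature item.
; CheckForCreature asks the camera manager's inventory component for the given item, printing a hint string if it is missing.
; When found, BalanceBalanceScale swaps the unbalanced scale for the balanced one, plays a creature noise and triggers the special lab drawer's interaction.
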(event Custom|BalanceBalanceScale
  (Rendering|SetActorHiddenInGame (Variables|Default|GetUnbalancedScale) true)
  (Rendering|SetActorHiddenInGame (Variables|Default|GetBalancedScale) false)
  (Audio|PlaySoundatLocation "/Game/Audio/CreatureNoise.CreatureNoise" (Transformation|GetActorLocation) "0, 0, 0" 1.0 1.0 0.0 0 0 0 0)
  (bind _returnvalue (Actor|GetActorOfClass "/Game/Blueprints/Lab/BP_LabDrawerSpecialOpen2.BP_LabDrawerSpecialOpen2_C"))
  (Default|InteractwithDrawer _returnvalue))

(event EventBeginPlay)

(event Collision|EventActorBeginOverlap
  (params (OtherActor :type Actor%20Object%20Reference)))

(event EventTick
  (params (DeltaSeconds :type Float%20%28single-precision%29)))

(fn ConstructionScript)

(fn CheckforCreature
  (params (ItemToCheck :type String))
  (bind _returnvalue (Actor|GetActorOfClass "/Game/Blueprints/BP_CameraManager.BP_CameraManager_C"))
  (bind _hasitem (Default|CheckInventoryforItem (Variables|/Game/Blueprints/BP_CameraManager.BP_CameraManager_C|GetBPC_Inventory _returnvalue) ItemToCheck))
  (if _hasitem
    (CallFunction|BalanceBalanceScale)
    (return ItemToCheck)
    (else
      (Development|PrintString "Hmm... balance scale..."))))