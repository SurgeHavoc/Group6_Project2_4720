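; A lockable lab drawer that opens when the player has the required item, and spawns an actor on that first opening.
; CheckForItem queries the inventory on BP_CameraManager while locked, then calls InteractWithDrawer to unlock, slide the Cube out and, after a short delay, spawn once at the Scene component.
; Once unlocked, CheckForItem simply toggles the drawer open and closed with instant relative offsets.
; Hover and locked feedback use PrintString.
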(event OnBeginCursorOver(Cube)
  (params (TouchedComponent :type Primitive%20Component%20Object%20Reference))
  (Development|PrintString "A drawer."))

(event Custom|InteractWithDrawer
  (Variables|Default|SetIsLocked? false)
  (Transformation|AddRelativeLocation (Variables|Default|GetCube) "0.000000,80.000000,0.000000" false false)
  (Variables|Default|SetBIsMoved? true)
  (Utilities|FlowControl|Delay 0.2)
  (if (not (Variables|Default|GetBHasSpawned))
    (Game|SpawnActorfromClass "/Game/Blueprints/Lab/BP_Lightbulb.BP_Lightbulb_C" (Math|Transform|MakeTransform (Transformation|GetWorldLocation (Variables|Default|GetScene))) "Undefined" "MultiplyWithRoot" 0 0)
    (Variables|Default|SetBHasSpawned true)))

(event EventBeginPlay)

(event Collision|EventActorBeginOverlap
  (params (OtherActor :type Actor%20Object%20Reference)))

(event EventTick
  (params (DeltaSeconds :type Float%20%28single-precision%29)))

(fn ConstructionScript)

(fn CheckforItem
  (params (ItemToCheck :type String))
  (if (Variables|Default|GetIsLocked?)
    (bind _returnvalue (Actor|GetActorOfClass "/Game/Blueprints/BP_CameraManager.BP_CameraManager_C"))
    (bind _hasitem (Default|CheckInventoryforItem (Variables|/Game/Blueprints/BP_CameraManager.BP_CameraManager_C|GetBPC_Inventory _returnvalue) ItemToCheck))
    (if _hasitem
      (CallFunction|InteractwithDrawer)
      (return ItemToCheck)
      (else
        (Development|PrintString "Hmm, the drawer is locked...")))
    (elif (Variables|Default|GetBIsMoved?)
      (Transformation|AddRelativeLocation (Variables|Default|GetCube) "0.000000,-80.000000,0.000000" false false)
      (Variables|Default|SetBIsMoved? false)
      (else
        (Transformation|AddRelativeLocation (Variables|Default|GetCube) "0.000000,80.000000,0.000000" false false)
        (Variables|Default|SetBIsMoved? true)))))