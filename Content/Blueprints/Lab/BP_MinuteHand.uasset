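; BP_MinuteHand is a pickup item, named as a clock's minute hand, that starts hidden in game with collision disabled.
; Pick Up Item prints a debug message, calls DestroyItem and returns its Item variable to the caller.
; DestroyItem plays a 2D pickup sound and destroys the actor after a short delay.
; Nothing in this Blueprint re-shows the actor or re-enables its collision.
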(event Custom|Destroy%20Item
  (Audio|PlaySound2D "/Game/Audio/PickupSound.PickupSound" 1.0 1.0 0.0 0 0)
  (Utilities|FlowControl|Delay 0.1)
  (Actor|DestroyActor))

(event EventBeginPlay
  (Rendering|SetActorHiddenInGame true)
  (Collision|SetActorEnableCollision false))

(event Collision|EventActorBeginOverlap
  (params (OtherActor :type Actor%20Object%20Reference)))

(fn ConstructionScript)

(fn PickUpItem
  (Development|PrintString "Item picked!")
  (CallFunction|DestroyItem)
  (return (Variables|Default|Getitem)))