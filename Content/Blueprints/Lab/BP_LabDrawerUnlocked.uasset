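; Lab drawer actor that slides open and shut on InteractWithDrawer and prints a description on cursor hover.
; Unlocked interactions toggle the Cube back and forth along its local Y axis, tracked by BIsMoved.
; While IsLocked is set, interaction waits briefly, spawns a BP_Beaker once at the Scene component, clears the lock and re-calls itself to slide.
; CheckForItem is a pass-through that returns its input.
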(event OnBeginCursorOver(Cube)
  (params (TouchedComponent :type Primitive%20Component%20Object%20Reference))
  (Development|PrintString "A drawer."))

(event Custom|InteractWithDrawer
  (if (Variables|Default|GetIsLocked?)
    (Utilities|FlowControl|Delay 0.2)
    (if (not (Variables|Default|GetBHasSpawned))
      (Game|SpawnActorfromClass "/Game/Blueprints/Lab/BP_Beaker.BP_Beaker_C" (Math|Transform|MakeTransform (Transformation|GetWorldLocation (Variables|Default|GetScene))) "Undefined" "MultiplyWithRoot" 0 0)
      (Variables|Default|SetBHasSpawned true)
      (Variables|Default|SetIsLocked? false)
      (CallFunction|InteractwithDrawer))
    (elif (Variables|Default|GetBIsMoved?)
      (Transformation|AddRelativeLocation (Variables|Default|GetCube) "0.000000,-80.000000,0.000000" false false)
      (Variables|Default|SetBIsMoved? false)
      (else
        (Transformation|AddRelativeLocation (Variables|Default|GetCube) "0.000000,80.000000,0.000000" false false)
        (Variables|Default|SetBIsMoved? true)))))

(event EventBeginPlay)

(event Collision|EventActorBeginOverlap
  (params (OtherActor :type Actor%20Object%20Reference)))

(event EventTick
  (params (DeltaSeconds :type Float%20%28single-precision%29)))

(fn ConstructionScript)

(fn CheckforItem
  (params (ItemToCheck :type String))
  (return ItemToCheck))