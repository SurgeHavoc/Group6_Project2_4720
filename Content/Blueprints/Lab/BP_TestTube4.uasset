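; BP_TestTube4 is a fillable test tube in the lab's test tube puzzle.
; CheckForBeaker looks up the given item in the inventory component on BP_CameraManager and prints a hint that a beaker is needed if it is missing.
; When the item is found, FillTestTube reveals the liquid mesh, then the tube increments the filled count on BP_TestTubePuzzle and calls its completion check.
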(event Custom|FillTestTube
  (Rendering|SetVisibility (Variables|Default|GetTest%20Tube%20Liquid) true false))

(event EventBeginPlay)

(event Collision|EventActorBeginOverlap
  (params (OtherActor :type Actor%20Object%20Reference)))

(fn ConstructionScript)

(fn CheckforBeaker
  (params (ItemToCheck :type String))
  (bind _returnvalue (Actor|GetActorOfClass "/Game/Blueprints/BP_CameraManager.BP_CameraManager_C"))
  (bind _hasitem (Default|CheckInventoryforItem (Variables|/Game/Blueprints/BP_CameraManager.BP_CameraManager_C|GetBPC_Inventory _returnvalue) ItemToCheck))
  (if _hasitem
    (CallFunction|FillTestTube)
    (bind _returnvalue_2 (Actor|GetActorOfClass "/Game/Blueprints/Lab/BP_TestTubePuzzle.BP_TestTubePuzzle_C"))
    (Math|Integer|IncrementInt (Variables|/Game/Blueprints/Lab/BP_TestTubePuzzle.BP_TestTubePuzzle_C|GetTestTubesFilled _returnvalue_2)
      (:%20%20
        (Default|CheckifFilled _returnvalue_2)
        (return ItemToCheck)))
    (else
      (Development|PrintString "You need a beaker to fill this test tube!"))))