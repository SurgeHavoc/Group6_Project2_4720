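; Clock puzzle actor in the Lab that activates once the player's inventory holds both minute and hour hands, then opens a linked door.
; CheckForClockHand queries BP_CameraManager's inventory and reveals both hands.
; Clicking either hand trigger runs one shared sequence: snap Cube and Sphere to fixed rotations, play a ghost sound, swing ClockDoorReference open in delayed steps.
; Cursor hover on each trigger sets flags on BP_CameraManager.
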(event OnClicked(MinuteHandTrigger)
  (params (TouchedComponent :type Primitive%20Component%20Object%20Reference) (ButtonPressed :type Key%20Structure :default "None"))
  (CallFunction|RotateMinuteHand))

(event OnBeginCursorOver(MinuteHandTrigger)
  (params (TouchedComponent :type Primitive%20Component%20Object%20Reference))
  (bind _returnvalue (Actor|GetActorOfClass "/Game/Blueprints/BP_CameraManager.BP_CameraManager_C"))
  (Variables|/Game/Blueprints/BP_CameraManager.BP_CameraManager_C|SetIsHoveringMinuteHandTrigger? _returnvalue true))

(event OnEndCursorOver(MinuteHandTrigger)
  (params (TouchedComponent :type Primitive%20Component%20Object%20Reference))
  (bind _returnvalue (Actor|GetActorOfClass "/Game/Blueprints/BP_CameraManager.BP_CameraManager_C"))
  (Variables|/Game/Blueprints/BP_CameraManager.BP_CameraManager_C|SetIsHoveringMinuteHandTrigger? _returnvalue false))

(event OnClicked(HourHandTrigger)
  (params (TouchedComponent :type Primitive%20Component%20Object%20Reference) (ButtonPressed :type Key%20Structure :default "None"))
  (CallFunction|RotateHourHand))

(event OnBeginCursorOver(HourHandTrigger)
  (params (TouchedComponent :type Primitive%20Component%20Object%20Reference))
  (bind _returnvalue (Actor|GetActorOfClass "/Game/Blueprints/BP_CameraManager.BP_CameraManager_C"))
  (Variables|/Game/Blueprints/BP_CameraManager.BP_CameraManager_C|SetIsHoveringHourHandTrigger? _returnvalue true))

(event OnEndCursorOver(HourHandTrigger)
  (params (TouchedComponent :type Primitive%20Component%20Object%20Reference))
  (bind _returnvalue (Actor|GetActorOfClass "/Game/Blueprints/BP_CameraManager.BP_CameraManager_C"))
  (Variables|/Game/Blueprints/BP_CameraManager.BP_CameraManager_C|SetIsHoveringHourHandTrigger? _returnvalue false))

(event Custom|RotateHourHand
  (if (Variables|Default|GetIsClockPuzzleActive?)
    (Transformation|SetRelativeRotation (Variables|Default|GetCube) "270.000000,0.000000,0.000000" false false)
    (Utilities|FlowControl|Delay 0.2)
    (Transformation|SetRelativeRotation (Variables|Default|GetSphere) "0.000000,0.000000,0.000000" false false)
    (Utilities|FlowControl|Delay 0.2)
    (CallFunction|OpenDoor)
    (else
      (Development|PrintString "Clock Puzzle not active yet!"))))

(event Custom|OpenDoor
  (bind _clockdoorreference (Variables|Default|GetClockDoorReference))
  (bind _anchorcube (Variables|/Game/Blueprints/Lab/BP_ClockDoor.BP_ClockDoor_C|GetAnchorCube _clockdoorreference))
  (bind _returnvalue (Components|GetChildComponent _anchorcube 0))
  (Audio|PlaySoundatLocation "/Game/Audio/ghost.ghost" (Transformation|GetActorLocation) "0, 0, 0" 1.0 1.0 0.0 0 0 0 0)
  (Transformation|AddLocalRotation _returnvalue "0.000000,30.000000,0.000000" false false)
  (Utilities|FlowControl|Delay 0.2)
  (Transformation|AddLocalRotation _returnvalue "0.000000,30.000000,0.000000" false false)
  (Utilities|FlowControl|Delay 0.2)
  (Transformation|AddLocalRotation _returnvalue "0.000000,30.000000,0.000000" false false))

(event Custom|ActivateClock
  (Variables|Default|SetIsClockPuzzleActive? true)
  (Rendering|SetVisibility (Variables|Default|GetMinute%20Hand) true false)
  (Rendering|SetVisibility (Variables|Default|GetHour%20Hand) true false))

(event Custom|RotateMinuteHand
  (if (Variables|Default|GetIsClockPuzzleActive?)
    (Transformation|SetRelativeRotation (Variables|Default|GetCube) "270.000000,0.000000,0.000000" false false)
    (Utilities|FlowControl|Delay 0.2)
    (Transformation|SetRelativeRotation (Variables|Default|GetSphere) "0.000000,0.000000,0.000000" false false)
    (Utilities|FlowControl|Delay 0.2)
    (CallFunction|OpenDoor)
    (else
      (Development|PrintString "Clock Puzzle not active yet!"))))

(event EventBeginPlay)

(event Collision|EventActorBeginOverlap
  (params (OtherActor :type Actor%20Object%20Reference)))

(fn ConstructionScript)

(fn CheckforClockHand
  (params (ItemToCheck :type String))
  (bind _returnvalue (Actor|GetActorOfClass "/Game/Blueprints/BP_CameraManager.BP_CameraManager_C"))
  (bind _hasitem (Default|CheckInventoryforItem (Variables|/Game/Blueprints/BP_CameraManager.BP_CameraManager_C|GetBPC_Inventory _returnvalue) "Minute Hand"))
  (if _hasitem
    (bind _hasitem_2 (Default|CheckInventoryforItem (Variables|/Game/Blueprints/BP_CameraManager.BP_CameraManager_C|GetBPC_Inventory _returnvalue) "Hour Hand"))
    (if _hasitem_2
      (CallFunction|ActivateClock)
      (return ItemToCheck)
      (else
        (Development|PrintString "Need an hour hand!")))
    (else
      (Development|PrintString "Need a minute hand!"))))