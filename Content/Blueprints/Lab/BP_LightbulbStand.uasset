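; BP_LightbulbStand is a lab puzzle stand that lights a bulb when the inventory holds the required item.
; CheckForLightbulb queries the inventory component on BP_CameraManager, triggering LightUpLightbulb on success or printing a balance-scale message otherwise.
; LightUpLightbulb reveals the bulb, then after a short delay plays a rock-breaking sound, swaps the bulb material and calls InteractWithDrawer on BP_LabDrawerSpecialOpen3.
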(event Custom|LightUpLightbulb
  (Rendering|SetVisibility (Variables|Default|GetLightbulb) true false)
  (Utilities|FlowControl|Delay 0.5)
  (Audio|PlaySoundatLocation "/Game/Audio/rock_breaking.rock_breaking" (Transformation|GetActorLocation) "0, 0, 0" 1.0 1.0 0.0 0 0 0 0)
  (Rendering|Material|SetMaterial (Variables|Default|GetLightbulb) 0 "/Game/Materials/M_LightBulb.M_LightBulb")
  (bind _returnvalue (Actor|GetActorOfClass "/Game/Blueprints/Lab/BP_LabDrawerSpecialOpen3.BP_LabDrawerSpecialOpen3_C"))
  (Default|InteractwithDrawer _returnvalue))

(event EventBeginPlay)

(event Collision|EventActorBeginOverlap
  (params (OtherActor :type Actor%20Object%20Reference)))

(event EventTick
  (params (DeltaSeconds :type Float%20%28single-precision%29)))

(fn ConstructionScript)

(fn CheckforLightbulb
  (params (ItemToCheck :type String))
  (bind _returnvalue (Actor|GetActorOfClass "/Game/Blueprints/BP_CameraManager.BP_CameraManager_C"))
  (bind _hasitem (Default|CheckInventoryforItem (Variables|/Game/Blueprints/BP_CameraManager.BP_CameraManager_C|GetBPC_Inventory _returnvalue) ItemToCheck))
  (if _hasitem
    (CallFunction|LightUpLightbulb)
    (return ItemToCheck)
    (else
      (Development|PrintString "Hmm... balance scale..."))))