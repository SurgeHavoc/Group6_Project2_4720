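; BP_AirVent is a lab air vent that opens when the player has a screwdriver, revealing a hidden minute hand.
; CheckForScrewdriver queries the inventory on BP_CameraManager and either triggers InteractWithAirVent or prints a hint.
; The interaction enables the minute hand, drops four screws and the cover through staggered physics simulation, disables the box collision and plays a breaking sound.
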(event Custom|InteractWithAirVent
  (bind _minutehandreference (Variables|Default|GetMinuteHandReference))
  (Rendering|SetActorHiddenInGame _minutehandreference false)
  (Collision|SetActorEnableCollision _minutehandreference true)
  (Utilities|FlowControl|Delay 0.2)
  (Physics|SetSimulatePhysics (Variables|Default|GetScrew) true)
  (Utilities|FlowControl|Delay 1.0)
  (Physics|SetSimulatePhysics (Variables|Default|GetScrew1) true)
  (Utilities|FlowControl|Delay 1.5)
  (Physics|SetSimulatePhysics (Variables|Default|GetScrew2) true)
  (Utilities|FlowControl|Delay 1.0)
  (Physics|SetSimulatePhysics (Variables|Default|GetScrew3) true)
  (Utilities|FlowControl|Delay 0.2)
  (Physics|SetSimulatePhysics (Variables|Default|GetStaticMesh) true)
  (Collision|SetCollisionEnabled (Variables|Default|GetBox) "NoCollision")
  (Utilities|FlowControl|Delay 0.2)
  (Audio|PlaySoundatLocation "/Game/Audio/rock_breaking.rock_breaking" (Transformation|GetActorLocation) "0, 0, 0" 1.0 1.0 0.0 0 0 0 0))

(event EventBeginPlay)

(event Collision|EventActorBeginOverlap
  (params (OtherActor :type Actor%20Object%20Reference)))

(event EventTick
  (params (DeltaSeconds :type Float%20%28single-precision%29)))

(fn ConstructionScript)

(fn CheckforScrewdriver
  (params (ItemToCheck :type String))
  (bind _returnvalue (Actor|GetActorOfClass "/Game/Blueprints/BP_CameraManager.BP_CameraManager_C"))
  (bind _hasitem (Default|CheckInventoryforItem (Variables|/Game/Blueprints/BP_CameraManager.BP_CameraManager_C|GetBPC_Inventory _returnvalue) ItemToCheck))
  (if _hasitem
    (CallFunction|InteractwithAirVent)
    (return ItemToCheck)
    (else
      (Development|PrintString "You need a screwdriver for the air vent!"))))