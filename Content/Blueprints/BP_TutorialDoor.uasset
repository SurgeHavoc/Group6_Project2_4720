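; BP_TutorialDoor is a clickable tutorial door that takes the player to Study_Map when they hold the tutorial key.
; Clicking its Cube looks up the key through the BP_GlobalInventory game instance, repeating the same CheckInventory call for each inventory entry.
; If found, it sets BHasKey, removes the key and opens the level.
; Otherwise it prints a message that a key is needed.
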(event OnClicked(Cube)
  (params (TouchedComponent :type Primitive%20Component%20Object%20Reference) (ButtonPressed :type Key%20Structure :default "None"))
  (bind _asbp_global_inventory (Utilities|Casting|CastToBP_GlobalInventory (Game|GetGameInstance)))
  (for _array_element (Variables|/Game/Blueprints/BP_Global/BP_GlobalInventory.BP_GlobalInventory_C|GetInventoryArray _asbp_global_inventory)
    (bind _hasitem (Default|CheckInventory _asbp_global_inventory (Variables|/Game/Blueprints/BP_Global/BP_GlobalInventory.BP_GlobalInventory_C|GetTutorialKeyReference _asbp_global_inventory))))
  (if _hasitem
    (Variables|Default|SetBHasKey true)
    (Default|RemovefromInventory _asbp_global_inventory (Variables|/Game/Blueprints/BP_Global/BP_GlobalInventory.BP_GlobalInventory_C|GetTutorialKeyReference _asbp_global_inventory))
    (Game|OpenLevel(byObjectReference) "/Game/Maps/Study_Map.Study_Map")
    (else
      (Development|PrintString "A key is needed to open this door!"))))

(event EventBeginPlay)

(event Collision|EventActorBeginOverlap
  (params (OtherActor :type Actor%20Object%20Reference)))

(event EventTick
  (params (DeltaSeconds :type Float%20%28single-precision%29)))

(fn ConstructionScript)