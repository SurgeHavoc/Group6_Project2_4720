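; Camera manager actor that cycles the player's view between four fixed cameras and handles related player input.
; Next and previous events wrap an index and activate only the matching camera, calling BP_Curtains' IsPlayerAway on Study_Map for all but the third.
; BeginPlay enables mouse events, sets the first view and shows an animated tutorial widget on the Tutorial level.
; Axis input nudges the mouse cursor, and Pause opens a menu and pauses the game.
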(event Custom|SwitchToNextCamera
  ;[1 1 1] Depending on input, switch the camera.
  (Math|Integer|IncrementInt (Variables|Default|GetCurrentCameraIndex)
    (:%20%20
      (if (> (Variables|Default|GetCurrentCameraIndex) 3)
        (Variables|Default|SetCurrentCameraIndex 0)
        (Development|PrintString (Utilities|String|ToString(Integer) (Variables|Default|GetCurrentCameraIndex)))
        (else
          (Development|PrintString (Utilities|String|ToString(Integer) (Variables|Default|GetCurrentCameraIndex)))))
      (switch int (Variables|Default|GetCurrentCameraIndex)
        (:0
          (Variables|Default|SetIsCamera1Active? true)
          (Components|Activation|SetActive (Variables|Default|GetCamera1) true false)
          (Components|Activation|SetActive (Variables|Default|GetCamera2) false false)
          (Components|Activation|SetActive (Variables|Default|GetCamera3) false false)
          (Components|Activation|SetActive (Variables|Default|GetCamera4) false false)
          (bind _returnvalue (Game|GetCurrentLevelName true))
          (if (Utilities|Enum|Equal(Enum) _returnvalue "Study_Map")
            (bind _returnvalue_2 (Actor|GetActorOfClass "/Game/Blueprints/BP_Study/BP_Curtains.BP_Curtains_C"))
            (Default|IsPlayerAway? _returnvalue_2)))
        (:1
          (Variables|Default|SetIsCamera1Active? false)
          (Components|Activation|SetActive (Variables|Default|GetCamera1) false false)
          (Components|Activation|SetActive (Variables|Default|GetCamera2) true false)
          (Components|Activation|SetActive (Variables|Default|GetCamera3) false false)
          (Components|Activation|SetActive (Variables|Default|GetCamera4) false false)
          (bind _returnvalue_3 (Game|GetCurrentLevelName true))
          (if (Utilities|Enum|Equal(Enum) _returnvalue_3 "Study_Map")
            (bind _returnvalue_4 (Actor|GetActorOfClass "/Game/Blueprints/BP_Study/BP_Curtains.BP_Curtains_C"))
            (Default|IsPlayerAway? _returnvalue_4)))
        (:2
          (Components|Activation|SetActive (Variables|Default|GetCamera1) false false)
          (Components|Activation|SetActive (Variables|Default|GetCamera2) false false)
          (Components|Activation|SetActive (Variables|Default|GetCamera3) true false)
          (Components|Activation|SetActive (Variables|Default|GetCamera4) false false))
        (:3
          (Variables|Default|SetIsCamera1Active? false)
          (Components|Activation|SetActive (Variables|Default|GetCamera1) false false)
          (Components|Activation|SetActive (Variables|Default|GetCamera2) false false)
          (Components|Activation|SetActive (Variables|Default|GetCamera3) false false)
          (Components|Activation|SetActive (Variables|Default|GetCamera4) true false)
          (bind _returnvalue_5 (Game|GetCurrentLevelName true))
          (if (Utilities|Enum|Equal(Enum) _returnvalue_5 "Study_Map")
            (bind _returnvalue_6 (Actor|GetActorOfClass "/Game/Blueprints/BP_Study/BP_Curtains.BP_Curtains_C"))
            (Default|IsPlayerAway? _returnvalue_6)))))))

(event Custom|SwitchToPreviousCamera
  ;[1 1 1] Depending on input, switch the camera.
  (Math|Integer|DecrementInt (Variables|Default|GetCurrentCameraIndex)
    (:%20%20
      (if (< (Variables|Default|GetCurrentCameraIndex) 0)
        (Variables|Default|SetCurrentCameraIndex 3)
        (Development|PrintString (Utilities|String|ToString(Integer) (Variables|Default|GetCurrentCameraIndex)))
        (else
          (Development|PrintString (Utilities|String|ToString(Integer) (Variables|Default|GetCurrentCameraIndex)))))
      (switch int (Variables|Default|GetCurrentCameraIndex)
        (:0
          (Variables|Default|SetIsCamera1Active? true)
          (Components|Activation|SetActive (Variables|Default|GetCamera1) true false)
          (Components|Activation|SetActive (Variables|Default|GetCamera2) false false)
          (Components|Activation|SetActive (Variables|Default|GetCamera3) false false)
          (Components|Activation|SetActive (Variables|Default|GetCamera4) false false)
          (bind _returnvalue (Game|GetCurrentLevelName true))
          (if (Utilities|Enum|Equal(Enum) _returnvalue "Study_Map")
            (bind _returnvalue_2 (Actor|GetActorOfClass "/Game/Blueprints/BP_Study/BP_Curtains.BP_Curtains_C"))
            (Default|IsPlayerAway? _returnvalue_2)))
        (:1
          (Variables|Default|SetIsCamera1Active? false)
          (Components|Activation|SetActive (Variables|Default|GetCamera1) false false)
          (Components|Activation|SetActive (Variables|Default|GetCamera2) true false)
          (Components|Activation|SetActive (Variables|Default|GetCamera3) false false)
          (Components|Activation|SetActive (Variables|Default|GetCamera4) false false)
          (bind _returnvalue_3 (Game|GetCurrentLevelName true))
          (if (Utilities|Enum|Equal(Enum) _returnvalue_3 "Study_Map")
            (bind _returnvalue_4 (Actor|GetActorOfClass "/Game/Blueprints/BP_Study/BP_Curtains.BP_Curtains_C"))
            (Default|IsPlayerAway? _returnvalue_4)))
        (:2
          (Components|Activation|SetActive (Variables|Default|GetCamera1) false false)
          (Components|Activation|SetActive (Variables|Default|GetCamera2) false false)
          (Components|Activation|SetActive (Variables|Default|GetCamera3) true false)
          (Components|Activation|SetActive (Variables|Default|GetCamera4) false false))
        (:3
          (Variables|Default|SetIsCamera1Active? false)
          (Components|Activation|SetActive (Variables|Default|GetCamera1) false false)
          (Components|Activation|SetActive (Variables|Default|GetCamera2) false false)
          (Components|Activation|SetActive (Variables|Default|GetCamera3) false false)
          (Components|Activation|SetActive (Variables|Default|GetCamera4) true false)
          (bind _returnvalue_5 (Game|GetCurrentLevelName true))
          (if (Utilities|Enum|Equal(Enum) _returnvalue_5 "Study_Map")
            (bind _returnvalue_6 (Actor|GetActorOfClass "/Game/Blueprints/BP_Study/BP_Curtains.BP_Curtains_C"))
            (Default|IsPlayerAway? _returnvalue_6)))))))

(event Collision|EventActorBeginOverlap
  (params (OtherActor :type Actor%20Object%20Reference)))

(event EventTick
  (params (DeltaSeconds :type Float%20%28single-precision%29))
  ;[1 1 1] Depending on input, switch the camera.
)

(event EventBeginPlay
  (bind _returnvalue (Game|GetPlayerController 0))
  ;[1 1 1] Set first camera to be active.
  (Input|EnableInput _returnvalue)
  (Variables|/Script/Engine.PlayerController|SetbEnableClickEvents _returnvalue true)
  (Variables|/Script/Engine.PlayerController|SetbEnableMouseOverEvents _returnvalue true)
  (Components|Activation|SetActive (Variables|Default|GetCamera1) true false)
  (Game|Player|SetViewTargetwithBlend (Game|GetPlayerController 0) (Components|GetOwner (Variables|Default|GetCamera1)) 0.0 "VTBlend_Linear" 0.0 false)
  (Components|Activation|SetActive (Variables|Default|GetCamera2) false false)
  (Components|Activation|SetActive (Variables|Default|GetCamera3) false false)
  (Components|Activation|SetActive (Variables|Default|GetCamera4) false false)
  (bind _returnvalue_2 (Game|GetCurrentLevelName true))
  (if (Utilities|Enum|Equal(Enum) _returnvalue_2 "Tutorial")
    (bind _returnvalue_3 (UserInterface|CreateWidget "/Game/UI/TutorialUI.TutorialUI_C"))
    (bind _output_get (Variables|Default|SetTutOnlyRef _returnvalue_3))
    (UserInterface|Viewport|AddtoViewport _output_get 0)
    (Default|PlayNotificationAnimation _output_get)))

(event Input|ActionEvents|InputActionPause
  (params (Key :type Key%20Structure :default "None"))
  (bind _returnvalue (Game|GetPlayerController 0))
  (:Pressed
    (bind _returnvalue_2 (UserInterface|CreateWidget "/Game/UI/PauseMenu.PauseMenu_C"))
    (UserInterface|Viewport|AddtoViewport _returnvalue_2 0)
    (Input|SetInputModeUIOnly _returnvalue 0 "DoNotLock" false)
    (Variables|/Script/Engine.PlayerController|SetbShowMouseCursor _returnvalue true)
    (Game|SetGamePaused true)))

(event Input|AxisEvents|InputAxisMouse2D
  (params (AxisValue :type Float%20%28single-precision%29))
  (bind _returnvalue (Game|GetPlayerController 0))
  (bind _returnvalue_2 (Input|AxisValues|GetMove_Cursor_X))
  (bind _returnvalue_3 (Input|AxisValues|GetMoveCursor_Y))
  (bind (_locationx _locationy) (Game|Player|GetMousePosition _returnvalue))
  (if (or (> (Math|Float|Absolute(Float) _returnvalue_2) 0.0) (> (Math|Float|Absolute(Float) _returnvalue_3) 0.0))
    (Class|PlayerController|SetMouseLocation (Game|GetPlayerController 0) (Math|Float|Round (+ (* _returnvalue_2 (Class|Actor|GetInputAxisKeyValue)) _locationx)) (Math|Float|Round (+ (* _returnvalue_3 (Class|Actor|GetInputAxisKeyValue)) _locationy)))))

(fn ConstructionScript)