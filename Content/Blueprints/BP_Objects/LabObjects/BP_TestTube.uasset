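; BP_TestTube is a clickable lab object that the player fills using a beaker from the inventory.
; Clicking its Cylinder checks BP_GlobalInventory, a Game Instance, for the beaker reference.
; With a beaker and an empty tube, it sets the filled flag, turns the material blue and removes the beaker from inventory.
; Otherwise it prints that the tube is already filled or needs a beaker.
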(event OnClicked(Cylinder)
  (params (TouchedComponent :type Primitive%20Component%20Object%20Reference) (ButtonPressed :type Key%20Structure))
  (bind _asbp_global_inventory (Utilities|Casting|CastToBP_GlobalInventory (Game|GetGameInstance)))
  (for _array_element (Variables|/Game/Blueprints/BP_Global/BP_GlobalInventory.BP_GlobalInventory_C|GetInventoryArray _asbp_global_inventory)
    (bind _hasitem (Default|CheckInventory _asbp_global_inventory (Variables|/Game/Blueprints/BP_Global/BP_GlobalInventory.BP_GlobalInventory_C|GetBeakerReference _asbp_global_inventory))))
  (if _hasitem
    (if (Variables|Default|GetBIsFilled)
      (Development|PrintString "Test Tube has been filled already!")
      (else
        (Variables|Default|SetBIsFilled true)
        (Rendering|Material|SetMaterial (Variables|Default|GetCylinder) 0 "/Game/Materials/Blue.Blue")
        (Default|RemovefromInventory _asbp_global_inventory (Variables|/Game/Blueprints/BP_Global/BP_GlobalInventory.BP_GlobalInventory_C|GetBeakerReference _asbp_global_inventory))))
    (else
      (Development|PrintString "You need a beaker to fill this test tube!"))))

(event EventBeginPlay)

(event Collision|EventActorBeginOverlap
  (params (OtherActor :type Actor%20Object%20Reference)))

(event EventTick
  (params (DeltaSeconds :type Float%20%28single-precision%29)))

(fn ConstructionScript)