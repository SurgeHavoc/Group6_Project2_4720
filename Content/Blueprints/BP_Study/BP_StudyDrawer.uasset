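; BP_StudyDrawer is a clickable, lockable drawer in the study that hides a note behind a key.
; Clicking it while locked checks the GameInstance inventory (BP_GlobalInventory) for the study drawer key, then consumes it or prints that one is needed.
; Unlocking slides the drawer out and, after a short delay, spawns BP_Note once with a small upward impulse.
; Later clicks toggle it open and closed with instant relative offsets; hovering prints a description.
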(event OnClicked(Cube)
  (params (TouchedComponent :type Primitive%20Component%20Object%20Reference) (ButtonPressed :type Key%20Structure :default "None"))
  (if (Variables|Default|GetIsLocked?)
    (bind _asbp_global_inventory (Utilities|Casting|CastToBP_GlobalInventory (Game|GetGameInstance)))
    (for _array_element (Variables|/Game/Blueprints/BP_Global/BP_GlobalInventory.BP_GlobalInventory_C|GetInventoryArray _asbp_global_inventory)
      (bind _hasitem (Default|CheckInventory _asbp_global_inventory (Variables|/Game/Blueprints/BP_Global/BP_GlobalInventory.BP_GlobalInventory_C|GetStudyDrawerKeyReference _asbp_global_inventory)))
      (if _hasitem
        (Variables|Default|SetBHasKey true)))
    (if (Variables|Default|GetBHasKey)
      (Default|RemovefromInventory _asbp_global_inventory (Variables|/Game/Blueprints/BP_Global/BP_GlobalInventory.BP_GlobalInventory_C|GetStudyDrawerKeyReference _asbp_global_inventory))
      (Variables|Default|SetIsLocked? false)
      (CallFunction|MoveDrawer)
      (Utilities|FlowControl|Delay 0.2)
      (if (not (Variables|Default|GetBHasSpawned))
        (bind _returnvalue (Game|SpawnActorfromClass "/Game/Blueprints/BP_Study/BP_Note.BP_Note_C" (Math|Transform|MakeTransform (Transformation|GetWorldLocation (Variables|Default|GetScene))) "Undefined" "MultiplyWithRoot" 0 0))
        (bind _output_get (Variables|Default|SetStudyNoteReference _returnvalue))
        (Variables|Default|SetBHasSpawned true)
        (Physics|AddImpulse (Variables|/Game/Blueprints/BP_Study/BP_Note.BP_Note_C|GetNote _output_get) "0.000000,0.000000,2.000000" "None" false))
      (else
        (Development|PrintString "A key is needed!")))
    (elif (Variables|Default|GetBIsMoved?)
      (CallFunction|MoveBackDrawer)
      (else
        (CallFunction|MoveDrawer)))))

(event OnBeginCursorOver(Cube)
  (params (TouchedComponent :type Primitive%20Component%20Object%20Reference))
  (Development|PrintString "A drawer."))

(event Custom|MoveDrawer
  (Transformation|AddRelativeLocation (Variables|Default|GetCube) "0.000000,50.000000,0.000000" false false)
  (Variables|Default|SetBIsMoved? true))

(event Custom|MoveBackDrawer
  (Transformation|AddRelativeLocation (Variables|Default|GetCube) "0.000000,-50.000000,0.000000" false false)
  (Variables|Default|SetBIsMoved? false))

(event EventBeginPlay)

(event Collision|EventActorBeginOverlap
  (params (OtherActor :type Actor%20Object%20Reference)))

(event EventTick
  (params (DeltaSeconds :type Float%20%28single-precision%29)))

(fn ConstructionScript)