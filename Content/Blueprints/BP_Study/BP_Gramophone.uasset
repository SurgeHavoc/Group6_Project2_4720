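; BP_Gramophone is a clickable study prop that trades a record from the player's inventory for a drawer key.
; Clicking its cube checks the game instance's BP_GlobalInventory for the record, printing a hint if it is missing.
; With the record, it removes the item and, only once, spawns BP_StudyDrawerKey at its location and launches it upward with an impulse.
; Hovering the cursor prints the prop's name.
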(event OnClicked(Cube)
  (params (TouchedComponent :type Primitive%20Component%20Object%20Reference) (ButtonPressed :type Key%20Structure :default "None"))
  (bind _asbp_global_inventory (Utilities|Casting|CastToBP_GlobalInventory (Game|GetGameInstance)))
  (for _array_element (Variables|/Game/Blueprints/BP_Global/BP_GlobalInventory.BP_GlobalInventory_C|GetInventoryArray _asbp_global_inventory)
    (bind _hasitem (Default|CheckInventory _asbp_global_inventory (Variables|/Game/Blueprints/BP_Global/BP_GlobalInventory.BP_GlobalInventory_C|GetRecordReference _asbp_global_inventory)))
    (if _hasitem
      (Variables|Default|SetBHasRecord true)))
  (if (Variables|Default|GetBHasRecord)
    (Default|RemovefromInventory _asbp_global_inventory (Variables|/Game/Blueprints/BP_Global/BP_GlobalInventory.BP_GlobalInventory_C|GetRecordReference _asbp_global_inventory))
    (if (not (Variables|Default|GetBHasSpawned))
      (bind _returnvalue (Game|SpawnActorfromClass "/Game/Blueprints/BP_Study/BP_StudyDrawerKey.BP_StudyDrawerKey_C" (Math|Transform|MakeTransform (Transformation|GetActorLocation)) "Undefined" "MultiplyWithRoot" 0 0))
      (bind _output_get (Variables|Default|SetDrawerKeyReference _returnvalue))
      (Variables|Default|SetBHasSpawned true)
      (Physics|AddImpulse (Variables|/Game/Blueprints/BP_Study/BP_StudyDrawerKey.BP_StudyDrawerKey_C|GetDrawerKey _output_get) "0.000000,0.000000,3000.000000" "None" false))
    (else
      (Development|PrintString "A record is needed!"))))

(event OnBeginCursorOver(Cube)
  (params (TouchedComponent :type Primitive%20Component%20Object%20Reference))
  (Development|PrintString "A gramophone!"))

(event EventBeginPlay)

(event Collision|EventActorBeginOverlap
  (params (OtherActor :type Actor%20Object%20Reference)))

(event EventTick
  (params (DeltaSeconds :type Float%20%28single-precision%29)))

(fn ConstructionScript)