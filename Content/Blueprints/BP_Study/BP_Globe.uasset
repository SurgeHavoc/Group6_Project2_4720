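; BP_Globe is a clickable globe puzzle in which the sphere's 90-degree turns must match a target sequence.
; BeginPlay builds that target from the Num variable plus fixed left/right codes.
; Clicking the sphere turns it left or right according to Option, recording each turn.
; CheckSequence runs inside each turn's debug-print loop, comparing once lengths match, then clearing the input and printing the result.
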(event OnClicked(Sphere)
  (params (TouchedComponent :type Primitive%20Component%20Object%20Reference) (ButtonPressed :type Key%20Structure :default "None"))
  (switch int (Variables|Default|GetOption)
    (:0
      (CallFunction|RotateLeft))
    (:1
      (CallFunction|RotateRight))))

(event Custom|RotateRight
  (Transformation|AddRelativeRotation (Variables|Default|GetSphere) "0.000000,90.000000,0.000000" false false)
  (Development|PrintString "Rotate Right!")
  (Utilities|Array|Add (Variables|Default|GetRotationSequence) 1)
  (for _array_element (Variables|Default|GetRotationSequence)
    (Development|PrintString (Utilities|String|ToString(Integer) _array_element))
    (CallFunction|CheckSequence)))

(event Custom|RotateLeft
  (Transformation|AddRelativeRotation (Variables|Default|GetSphere) "0.000000,-90.000000,0.000000" false false)
  (Development|PrintString "Rotate Left!")
  (Utilities|Array|Add (Variables|Default|GetRotationSequence) 0)
  (for _array_element (Variables|Default|GetRotationSequence)
    (Development|PrintString (Utilities|String|ToString(Integer) _array_element))
    (CallFunction|CheckSequence)))

(event EventBeginPlay
  (bind _output_get (Variables|Default|SetRotationSequence (Variables|Default|GetRotationSequence)))
  (Utilities|Array|Clear _output_get)
  (bind _output_get_2 (Variables|Default|SetCorrectSequence (Utilities|Array|MakeArray (Variables|Default|GetNum) 0 1 1 0 1)))
  (for _array_element _output_get_2
    (Development|PrintString (Utilities|String|ToString(Integer) _array_element))))

(event Collision|EventActorBeginOverlap
  (params (OtherActor :type Actor%20Object%20Reference)))

(event EventTick
  (params (DeltaSeconds :type Float%20%28single-precision%29)))

(fn ConstructionScript)

(fn CheckSequence
  (if (== (Utilities|Array|Length (Variables|Default|GetRotationSequence)) (Utilities|Array|Length (Variables|Default|GetCorrectSequence)))
    (Variables|Default|SetIsSequenceCorrect? true)
    (for (_array_element _array_index) (Variables|Default|GetRotationSequence)
      (if (not (== (Utilities|Array|Get(acopy) (Variables|Default|GetCorrectSequence) _array_index) _array_element))
        (Utilities|Array|Clear (Variables|Default|GetRotationSequence))
        (Variables|Default|SetIsSequenceCorrect? false)))
    (if (Variables|Default|GetIsSequenceCorrect?)
      (Utilities|Array|Clear (Variables|Default|GetRotationSequence))
      (Development|PrintString "Correct!")
      (else
        (Utilities|Array|Clear (Variables|Default|GetRotationSequence))
        (Development|PrintString "Try again!")))))