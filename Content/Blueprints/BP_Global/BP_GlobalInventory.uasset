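; BP_GlobalInventory is a simple inventory that stores items in a single InventoryArray.
; AddToInventory and RemoveFromInventory modify the array, then print the display name of every item it holds to the screen.
; CheckInventory returns whether a given item is in the array.
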(fn AddtoInventory
  (params (Item :type Actor%20Object%20Reference))
  (Utilities|Array|Add (Variables|Default|GetInventoryArray) Item)
  (for _array_element (Variables|Default|GetInventoryArray)
    (Development|PrintString (Utilities|GetDisplayName _array_element))))

(fn CheckInventory
  (params (ItemToCheck :type Actor%20Object%20Reference))
  (return (Utilities|Array|ContainsItem (Variables|Default|GetInventoryArray) ItemToCheck)))

(fn RemovefromInventory
  (params (ItemToRemove :type Actor%20Object%20Reference))
  (Utilities|Array|RemoveItem (Variables|Default|GetInventoryArray) ItemToRemove)
  (for _array_element (Variables|Default|GetInventoryArray)
    (Development|PrintString (Utilities|GetDisplayName _array_element))))