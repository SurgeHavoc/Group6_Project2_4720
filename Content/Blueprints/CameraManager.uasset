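; CameraManager cycles the first player controller's view through the level's switchable cameras.
; On BeginPlay it gathers every CameraActor tagged SwitchableCamera and stores the array and its count.
; Each SwitchToNextCamera call sets the view target to the camera at the current index, then advances the index, wrapping to zero after the last one.
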(event Custom|SwitchToNextCamera
  (Game|Player|SetViewTargetwithBlend (Game|GetPlayerController 0) (Utilities|Array|Get(acopy) (Variables|Default|GetCameraActors) (Variables|Default|GetCurrentCameraIndex)) 0.0 "VTBlend_Linear" 0.0 false)
  (Math|Integer|IncrementInt (Variables|Default|GetCurrentCameraIndex)
    (:%20%20
      (if (== (+ (Variables|Default|GetCurrentCameraIndex) 0) (Variables|Default|GetAmountOfCameras))
        (Variables|Default|SetCurrentCameraIndex 0)))))

(event EventBeginPlay
  (bind _outactors (Actor|GetAllActorsOfClasswithTag "/Script/Engine.CameraActor" "SwitchableCamera"))
  (bind _output_get (Variables|Default|SetCameraActors _outactors))
  (Variables|Default|SetAmountOfCameras (Utilities|Array|Length _output_get)))

(event Collision|EventActorBeginOverlap
  (params (OtherActor :type Actor%20Object%20Reference)))

(event EventTick
  (params (DeltaSeconds :type Float%20%28single-precision%29)))

(fn ConstructionScript)